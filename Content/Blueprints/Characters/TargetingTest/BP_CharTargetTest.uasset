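; BP_CharTargetTest is a test character for Tab-toggled targeting of other instances of its own class.
; On Tab, it line-traces to each instance and picks the lowest DistanceFromPlayerCheck among visible ones, within a threshold.
; TargetSelect flip-flops the chosen target's marker visibility, and pressing Tab again releases it.
; DistanceFromPlayerCheck measures to the last instance found, not explicitly the player; the Timeline-fed gate has no output logic.
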(event EventBeginPlay
  (bind _returnvalue (Game|GetPlayerController 0))
  (Input|SetInputModeGameandUI _returnvalue 0 "DoNotLock" true)
  (Variables|/Script/Engine.PlayerController|SetbShowMouseCursor _returnvalue true))

(event EventTargetSelect
  (bind _targetvisual (Variables|Default|GetTargetVisual))
  (Utilities|FlowControl|FlipFlop
    (:A
      (Development|SetHiddeninGame _targetvisual false false))
    (:B
      (Development|SetHiddeninGame _targetvisual true false))))

(event Input|KeyboardEvents|Tab
  (params (Key :type Key%20Structure :default "None"))
  (:Pressed
    (Variables|Default|SetClosestTargetDistance (Variables|Default|GetMinimumDistanceToEnable))
    (if (Variables|Default|GetbIsTargeting)
      (Variables|Default|SetbIsTargeting false)
      (Default|TargetSelect (Variables|Default|GetNearestTarget) :!label _label)
      (Utilities|FlowControl|Gate true) ; enters at Toggle
      (else
        (bind _outactors (Actor|GetAllActorsOfClass "BP_CharTargetTest_C"))
        (for _array_element _outactors
          (bind _outhit (Collision|LineTraceForObjects (Transformation|GetActorLocation) (Transformation|GetActorLocation _array_element) (Utilities|Array|MakeArray "ObjectTypeQuery1" "ObjectTypeQuery2" "ObjectTypeQuery3") false 0 "None"))
          (if (== _array_element (.HitActor (Collision|BreakHitResult _outhit)))
            (bind _distancefromplayer (CallFunction|DistancefromPlayerCheck _array_element))
            (Math|Float|CompareFloat _distancefromplayer (Variables|Default|GetClosestTargetDistance)
              (:<
                (Variables|Default|SetClosestTargetDistance _distancefromplayer)
                (Variables|Default|SetNearestTarget _array_element)))))
        (if (< (Variables|Default|GetClosestTargetDistance) (Variables|Default|GetMinimumDistanceToEnable))
          (Variables|Default|SetbIsTargeting true)
          (goto _label))))))

(fn ConstructionScript)

(fn DistancefromPlayerCheck
  (bind _outactors (Actor|GetAllActorsOfClass "BP_CharTargetTest_C"))
  (for _array_element _outactors
    _)
  (return (Transformation|GetDistanceTo _array_element)))